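; Pet actor that follows the ScrewMan player or moves to a magnet spot to suck in Score-tagged leaves.
; Once started, Tick lerps it toward the player's PetFollow point or MagnetPosition, depending on PetState.
; In Magnet state, MagnetCollision overlaps dynamically attach a MoveToPet component to each leaf.
; EatCollision overlaps, in any state, hide the leaf sprite and disable its collision.
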(event `self.ReceiveBeginPlay`
  (`KismetSystemLibrary.Delay` 0.2)
  (bind _outactors (`GameplayStatics.GetAllActorsOfClass` "/Game/BluePrints/ScrewManPawn.ScrewManPawn_C"))
  (set `self.FollowPosition` (`/Game/BluePrints/ScrewManPawn.PetFollow` (`KismetArrayLibrary.Array_Get` _outactors))))

(event `self.ReceiveActorBeginOverlap`
  (params (OtherActor :type "Actor Object Reference")))

(event `self.ReceiveTick`
  (params (DeltaSeconds :type "Float (single-precision)"))
  ;[1 1 1] 單純根據狀態決定移動到跟隨螺絲人的位置還是吸葉子的位置
  (if (`self.IsStart`)
    (`self.K2_SetActorLocation` (`KismetMathLibrary.VLerp` (`self.K2_GetActorLocation`) (select `/Game/BluePrints/EPetState` (`self.PetState`) :`NewEnumerator0` (`SceneComponent.K2_GetComponentLocation` (`self.FollowPosition`)) :`NewEnumerator1` (`self.K2_GetActorLocation` (`self.MagnetPosition`))) (* DeltaSeconds 3.0)))))

(event `self.MagnetCollision.OnComponentBeginOverlap`
  (params (OtherActor :type "Actor Object Reference") (OtherComp :type "PrimitiveComponent Object Reference") (OtherBodyIndex :type Integer) (bFromSweep :type Boolean) (SweepResult :type "HitResult Structure (by ref)"))
  (bind _componenttags (`ActorComponent.ComponentTags` OtherComp))
  (if (and (`|EnumEquality` (`self.PetState`) "NewEnumerator1") (> (`KismetArrayLibrary.Array_Length` _componenttags) 0))
    (if (== (`KismetArrayLibrary.Array_Get` _componenttags) "Score")
      ;[1 1 1] 將MoveToPet動態加到葉子身上
      (bind _returnvalue (`AddComponent|Move to Pet_2` :`self` OtherActor :`bManualAttachment` true))
      (`SceneComponent.K2_AttachTo` _returnvalue OtherComp "None" "KeepRelativeOffset" true)
      (set `/Game/BluePrints/MoveToPet.ParentComponent` OtherComp _returnvalue))))

(event `self.EatCollision.OnComponentBeginOverlap`
  (params (OtherActor :type "Actor Object Reference") (OtherComp :type "PrimitiveComponent Object Reference") (OtherBodyIndex :type Integer) (bFromSweep :type Boolean) (SweepResult :type "HitResult Structure (by ref)"))
  (bind _componenttags (`ActorComponent.ComponentTags` OtherComp))
  (if (> (`KismetArrayLibrary.Array_Length` _componenttags) 0)
    (if (== (`KismetArrayLibrary.Array_Get` _componenttags) "Score")
      ;[1 1 1] 寵物吃到葉子後，關掉Sprite的顯示還有碰撞
      (bind _aspaper_sprite_component (cast `PaperSpriteComponent` OtherComp))
      (`PrimitiveComponent.SetCollisionEnabled` _aspaper_sprite_component "NoCollision")
      (`SceneComponent.SetVisibility` _aspaper_sprite_component false false))))

(fn `UserConstructionScript`)