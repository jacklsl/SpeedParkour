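; Level generator that extends the level by spawning segments as its collision component overlaps markers tagged "End".
; Each overlap spawns a random obstacle or score segment at the marker's location, with obstacles listed twice in the selection to weight the odds.
; Once a randomized real-time timer expires, one random "Score" sprite (a leaf) in the new segment becomes a magnet through a sprite and tag swap, then the timer resets.
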(event `self.ReceiveBeginPlay`
  (set `self.CreateMangetTime` (+ (`GameplayStatics.GetRealTimeSeconds`) (`KismetMathLibrary.Conv_IntToDouble` (`KismetMathLibrary.RandomIntegerInRange` 10 20)))))

(event `self.CollisionComponent.OnComponentBeginOverlap`
  (params (OtherActor :type "Actor Object Reference") (OtherComp :type "PrimitiveComponent Object Reference") (OtherBodyIndex :type Integer) (bFromSweep :type Boolean) (SweepResult :type "HitResult Structure (by ref)"))
  (if (== (`KismetArrayLibrary.Array_Get` (`ActorComponent.ComponentTags` OtherComp)) "End")
    (bind _returnvalue (`|SpawnActorFromClass` (select `int` (`KismetMathLibrary.RandomInteger` 11) :`0` "/Game/Prefabs/Obstacle1.Obstacle1_C" :`1` "/Game/Prefabs/Obstacle2.Obstacle2_C" :`2` "/Game/Prefabs/Obstacle3.Obstacle3_C" :`3` "/Game/Prefabs/Score1.Score1_C" :`4` "/Game/Prefabs/Score2.Score2_C" :`5` "/Game/Prefabs/Score3.Score3_C" :`6` "/Game/Prefabs/Score4.Score4_C" :`7` "/Game/Prefabs/Score5.Score5_C" :`8` "/Game/Prefabs/Obstacle1.Obstacle1_C" :`9` "/Game/Prefabs/Obstacle2.Obstacle2_C" :`10` "/Game/Prefabs/Obstacle3.Obstacle3_C" :!type "Actor Class Reference") (`KismetMathLibrary.Conv_VectorToTransform` (`SceneComponent.K2_GetComponentLocation` OtherComp)) "AdjustIfPossibleButDontSpawnIfColliding" "OverrideRootScale"))
    ;[1 1 1] 生成磁鐵的方式為從某個葉子動態改成磁鐵
    (if (> (`GameplayStatics.GetRealTimeSeconds`) (`self.CreateMangetTime`))
      (bind _returnvalue_2 (`self.GetComponentsByTag` _returnvalue "/Script/Paper2D.PaperSpriteComponent" "Score"))
      (set `self.Index` (`KismetMathLibrary.RandomInteger` (`KismetArrayLibrary.Array_Length` _returnvalue_2)))
      (bind _item (`KismetArrayLibrary.Array_Get` _returnvalue_2 (`self.Index`)))
      (`PaperSpriteComponent.SetSprite` _item "/Game/Sprites/Magnet_Sprite.Magnet_Sprite")
      (set `ActorComponent.ComponentTags` (`|MakeArray` "Magnet" :!type "Name") _item)
      (set `self.CreateMangetTime` (+ (`GameplayStatics.GetRealTimeSeconds`) (`KismetMathLibrary.Conv_IntToDouble` (`KismetMathLibrary.RandomIntegerInRange` 15 30)))))))

(fn `UserConstructionScript`)