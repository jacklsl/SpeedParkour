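; Player pawn for ScrewMan, a runner game with jump, double jump, slide and death.
; Input changes the state held in ScrewManGameMode using timer windows for jumps, and Tick maps that state to flipbook animation and looping, easing the body back to its start on death.
; Tag-based overlaps collect score, kill on obstacles, or switch the pet's state for a timed magnet.
; The finished death animation reveals the HUD's reload widget.
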(event `self.ReceiveBeginPlay`
  (bind _asscrew_man_game_mode (cast `/Game/BluePrints/ScrewManGameMode` (`GameplayStatics.GetGameMode`)))
  (set `self.GameMode` _asscrew_man_game_mode)
  (set `self.OrginLocation` (`self.K2_GetActorLocation`))
  (bind _asscrew_man_hud (cast `/Game/Blueprints/ScrewManHUD` (`PlayerController.GetHUD` (`GameplayStatics.GetPlayerController` 0))))
  (set `self.HUD` _asscrew_man_hud)
  (bind _outactors (`GameplayStatics.GetAllActorsOfClass` "/Game/BluePrints/Pet_Blueprint.Pet_Blueprint_C"))
  (bind _output_get (set `self.Pet` (`KismetArrayLibrary.Array_Get` _outactors)))
  (`KismetSystemLibrary.Delay` 0.2)
  (set `/Game/BluePrints/Pet_Blueprint.IsStart` true _output_get))

(event `self.ReceiveTick`
  (params (DeltaSeconds :type "Float (single-precision)"))
  (bind _gamemode (`self.GameMode`))
  (bind _flipbook (`self.Flipbook`))
  (bind _screwmanstate (`/Game/BluePrints/ScrewManGameMode.ScrewManState` _gamemode))
  ;[1 1 1] 確保滑行動作只會在跑的動作之後啟動
  (if (`self.DoSlide`)
    (switch `/Game/BluePrints/EScrewManState` (`/Game/BluePrints/ScrewManGameMode.ScrewManState` (`self.GameMode`))
      (:`NewEnumerator0`
        (set `/Game/BluePrints/ScrewManGameMode.ScrewManState` "NewEnumerator3" _gamemode))
      (:`NewEnumerator4`
        (set `self.DoSlide` false)
        (`AudioComponent.Stop` (`self.SlideCue`)))))
  ;[1 1 1] 根據狀態決定要播放那個Flipbook
  (`PaperFlipbookComponent.SetFlipbook` _flipbook (select `/Game/BluePrints/EScrewManState` _screwmanstate :`NewEnumerator0` "/Game/Flipbook/redgirl/redgirl_run.redgirl_run" :`NewEnumerator1` "/Game/Flipbook/redgirl/redgirl_onejump.redgirl_onejump" :`NewEnumerator2` "/Game/Flipbook/redgirl/redgirl_doublejump.redgirl_doublejump" :`NewEnumerator3` "/Game/Flipbook/redgirl/redgirl_side.redgirl_side" :`NewEnumerator4` "/Game/Flipbook/redgirl/redgirl_side.redgirl_side" :!type "PaperFlipbook Object Reference"))
  ;[1 1 1] 控制Flipbook動畫是否循環播放
  (switch `/Game/BluePrints/EScrewManState` _screwmanstate
    (:`NewEnumerator0`
      (`PaperFlipbookComponent.SetLooping` _flipbook true :!label _label))
    (:`NewEnumerator1`
      (goto _label))
    (:`NewEnumerator2`
      (`PaperFlipbookComponent.SetLooping` _flipbook false :!label _label_2))
    (:`NewEnumerator3`
      (`AudioComponent.Play` (`self.SlideCue`) 0.0)
      (goto _label))
    (:`NewEnumerator4`
      ;[1 1 1] 確保死亡時一定會落在地面上
      (`self.K2_SetActorLocation` (`KismetMathLibrary.VLerp` (`self.K2_GetActorLocation`) (`self.OrginLocation`) 0.1))
      (goto _label_2)))
  (`PaperFlipbookComponent.Play` _flipbook))

(event `Character_Jump`
  (bind _gamemode (`self.GameMode`))
  (bind _timer (`/Game/BluePrints/ScrewManGameMode.Timer` (`self.GameMode`)))
  (switch `/Game/BluePrints/EScrewManState` (`/Game/BluePrints/ScrewManGameMode.ScrewManState` (`self.GameMode`)) :!label _label_3
    (:`NewEnumerator0`
      (`AudioComponent.Play` (`self.JumpAudio`) 0.0 :!label _label_4)
      (set `/Game/BluePrints/ScrewManGameMode.ScrewManState` "NewEnumerator1" _gamemode)
      (set `/Game/BluePrints/ScrewManGameMode.Timer` 0.0 _gamemode))
    (:`NewEnumerator1`
      (if (< _timer 0.55)
        (`AudioComponent.Play` (`self.JumpAudio`) 0.0)
        (set `/Game/BluePrints/ScrewManGameMode.ScrewManState` "NewEnumerator2" _gamemode)
        (else
          (if (> _timer 0.95) :!label _label_5
            (goto _label_4)))))
    (:`NewEnumerator2`
      (goto _label_5))))

(event `Key|LeftMouseButton`
  (params (Key :type "Key Structure" :default "AnyKey"))
  (:`Pressed`
    (goto _label_3)))

(event `Character_Slide`
  (switch `/Game/BluePrints/EScrewManState` (`/Game/BluePrints/ScrewManGameMode.ScrewManState` (`self.GameMode`)) :!label _label_6
    (:`NewEnumerator0`
      _)
    (:`NewEnumerator1`
      _)
    (:`NewEnumerator2`
      _))
  (set `self.DoSlide` true))

(event `Character_Run`
  (bind _gamemode (`self.GameMode`))
  (set `self.DoSlide` false :!label _label_7)
  (switch `/Game/BluePrints/EScrewManState` (`/Game/BluePrints/ScrewManGameMode.ScrewManState` _gamemode)
    (:`NewEnumerator3`
      (set `/Game/BluePrints/ScrewManGameMode.ScrewManState` "NewEnumerator0" _gamemode)
      (`AudioComponent.Stop` (`self.SlideCue`)))))

(event `Key|RightMouseButton`
  (params (Key :type "Key Structure" :default "AnyKey"))
  (:`Pressed`
    (goto _label_6))
  (:`Released`
    (goto _label_7)))

(event `self.Flipbook.OnComponentBeginOverlap`
  (params (OtherActor :type "Actor Object Reference") (OtherComp :type "PrimitiveComponent Object Reference") (OtherBodyIndex :type Integer) (bFromSweep :type Boolean) (SweepResult :type "HitResult Structure (by ref)"))
  (bind _componenttags (`ActorComponent.ComponentTags` OtherComp))
  (if (> (`KismetArrayLibrary.Array_Length` _componenttags) 0)
    (switch `name` (`KismetArrayLibrary.Array_Get` _componenttags)
      (:`Score`
        ;[1 1 1] 若碰到的是分數則隱藏Sprite的顯示並且關閉碰撞
        (bind _aspaper_sprite_component (cast `PaperSpriteComponent` OtherComp :!label _label_8))
        (`PrimitiveComponent.SetCollisionEnabled` _aspaper_sprite_component "NoCollision")
        (`SceneComponent.SetVisibility` _aspaper_sprite_component false false)
        (`AudioComponent.Play` (`self.EatAudio`) 0.0)
        (set `self.Score` (+ (`self.Score`) 1)))
      (:`Obstacle`
        ;[1 1 1] 若碰到的是障礙物則設定螺絲人狀態為Dead
        (set `/Game/BluePrints/ScrewManGameMode.ScrewManState` "NewEnumerator4" (`self.GameMode`))
        (`AudioComponent.Play` (`self.DeadAudio`) 0.0)
        (`AudioComponent.Stop` (`self.BGCue`)))
      (:`Magnet`
        (set `/Game/BluePrints/Pet_Blueprint.PetState` "NewEnumerator1" (`self.Pet`))
        (`KismetSystemLibrary.K2_SetTimer` null "EndMagnet" 5.0)
        (goto _label_8)))))

(event `self.Flipbook.OnFinishedPlaying`
  (switch `/Game/BluePrints/EScrewManState` (`/Game/BluePrints/ScrewManGameMode.ScrewManState` (`self.GameMode`))
    (:`NewEnumerator4`
      (`Widget.SetVisibility` (`/Game/Blueprints/ScrewManHUD.ReloadWidget` (`self.HUD`)) "Visible"))))

(fn `EndMagnet`
  (set `/Game/BluePrints/Pet_Blueprint.PetState` "NewEnumerator0" (`self.Pet`)))

(fn `UserConstructionScript`)