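; Actor component that drives the owner's vertical jump motion from the ScrewManGameMode state.
; On initialization it caches the game mode and the owner's starting Z.
; Each tick during a single or double jump, it advances the game mode's Timer, samples that jump's float curve and sets Z relative to the origin.
; A flag restarts the timer once when a double jump begins; after one second, the state returns to running.
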(event `self.ReceiveTick`
  (params (DeltaSeconds :type "Float (single-precision)"))
  (bind _returnvalue (`self.GetOwner`))
  (bind _gamemode (`self.GameMode`))
  (bind _gamemode_2 (`self.GameMode`))
  (bind (_returnvalue_x _returnvalue_y) (`KismetMathLibrary.BreakVector` (`Actor.K2_GetActorLocation` _returnvalue)))
  (bind _screwmanstate (`/Game/BluePrints/ScrewManGameMode.ScrewManState` (`self.GameMode`)))
  (switch `/Game/BluePrints/EScrewManState` _screwmanstate
    (:`NewEnumerator1`
      (set `self.IsTwoJumping` false))
    (:`NewEnumerator2`
      (if (not (`self.IsTwoJumping`))
        (set `/Game/BluePrints/ScrewManGameMode.Timer` 0.0 _gamemode_2)
        (set `self.IsTwoJumping` true))))
  (bind _output_get (set `/Game/BluePrints/ScrewManGameMode.Timer` (+ (`/Game/BluePrints/ScrewManGameMode.Timer` _gamemode_2) DeltaSeconds) _gamemode_2))
  (`Actor.K2_SetActorLocation` _returnvalue (`KismetMathLibrary.MakeVector` _returnvalue_x _returnvalue_y (+ (`CurveFloat.GetFloatValue` (select `/Game/BluePrints/EScrewManState` _screwmanstate :`NewEnumerator1` "/Game/Curve/OneJumpCurve.OneJumpCurve" :`NewEnumerator2` "/Game/Curve/TwoJumpCurve.TwoJumpCurve" :!type "CurveFloat Object Reference") _output_get) (`self.OrginZ`))) false)
  (if (>= (`/Game/BluePrints/ScrewManGameMode.Timer` _gamemode) 1.0)
    (set `/Game/BluePrints/ScrewManGameMode.Timer` 0.0 _gamemode)
    (set `self.IsTwoJumping` false)
    (switch `/Game/BluePrints/EScrewManState` (`/Game/BluePrints/ScrewManGameMode.ScrewManState` _gamemode)
      (:`NewEnumerator1`
        _)
      (:`NewEnumerator2`
        _))
    (set `/Game/BluePrints/ScrewManGameMode.ScrewManState` "NewEnumerator0" _gamemode)))

(event `self.ReceiveInitializeComponent`
  (bind (_returnvalue_x _returnvalue_y _returnvalue_z) (`KismetMathLibrary.BreakVector` (`Actor.K2_GetActorLocation` (`self.GetOwner`))))
  (bind _asscrew_man_game_mode (cast `/Game/BluePrints/ScrewManGameMode` (`GameplayStatics.GetGameMode`)))
  (set `self.GameMode` _asscrew_man_game_mode)
  (set `self.OrginZ` _returnvalue_z))