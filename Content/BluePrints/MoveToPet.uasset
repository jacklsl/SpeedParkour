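; MoveToPet is a component Blueprint that makes its parent component, a leaf according to the graph comment, fly toward the pet.
; On initialization it caches the first Pet_Blueprint actor found in the level.
; Each Tick lerps the parent's world location toward that actor's current location by a delta-time-scaled alpha, giving an eased homing motion without sweep collision.
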(event `self.ReceiveTick`
  (params (DeltaSeconds :type "Float (single-precision)"))
  ;[1 1 1] 讓葉子往寵物飛過去
  (`self.K2_SetWorldLocation` (`self.ParentComponent`) (`KismetMathLibrary.VLerp` (`self.K2_GetComponentLocation` (`self.ParentComponent`)) (`Actor.K2_GetActorLocation` (`self.Pet`)) (* DeltaSeconds 20.0)) false))

(event `self.ReceiveInitializeComponent`
  (bind _outactors (`GameplayStatics.GetAllActorsOfClass` "/Game/BluePrints/Pet_Blueprint.Pet_Blueprint_C"))
  (set `self.Pet` (`KismetArrayLibrary.Array_Get` _outactors)))