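; Movement component that automatically scrolls its owning actor left along the X axis in the ScrewMan game.
; BeginPlay caches the ScrewManGameMode, and Tick moves the owner only while its ScrewManState is running, jumping, double-jumping or sliding.
; Each step scales Speed by delta time, and the IsCycle flag applies a modulo to the new X so the actor loops over a fixed span.
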(event `self.ReceiveTick`
  (params (DeltaSeconds :type "Float (single-precision)"))
  (bind _returnvalue (`self.GetOwner`))
  (bind (_returnvalue_x _returnvalue_y _returnvalue_z) (`KismetMathLibrary.BreakVector` (`Actor.K2_GetActorLocation` _returnvalue)))
  (bind _returnvalue_2 (+ (* DeltaSeconds (`self.Speed`) (/ -800.0 20.0)) _returnvalue_x))
  ;[1 1 1] 自動往左移
  (switch `/Game/BluePrints/EScrewManState` (`/Game/BluePrints/ScrewManGameMode.ScrewManState` (`self.GameMode`))
    (:`NewEnumerator0`
      _)
    (:`NewEnumerator1`
      _)
    (:`NewEnumerator2`
      _)
    (:`NewEnumerator3`
      _))
  (`Actor.K2_SetActorLocation` _returnvalue (`KismetMathLibrary.MakeVector` (`KismetMathLibrary.SelectFloat` (mod _returnvalue_2 800.0) _returnvalue_2 (`self.IsCycle`)) _returnvalue_y _returnvalue_z) false false))

(event `self.ReceiveBeginPlay`
  (bind _asscrew_man_game_mode (cast `/Game/BluePrints/ScrewManGameMode` (`GameplayStatics.GetGameMode`)))
  (set `self.GameMode` _asscrew_man_game_mode))