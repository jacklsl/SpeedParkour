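; ScrewManHUD is a Blueprint that sets up on-screen widgets when play begins.
; It creates a ReloadUI widget, stores it and adds it hidden to the viewport, then adds an FpsUI widget.
; It also shows the mouse cursor for player controller 0.
; On EndPlay it removes every top-level UserWidget from its parent, not only the two it created.
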(event `self.ReceiveBeginPlay`
  (bind _returnvalue (`|CreateWidget` "/Game/BluePrints/ReloadUI.ReloadUI_C"))
  (bind _output_get (set `self.ReloadWidget` _returnvalue))
  (`Widget.SetVisibility` _output_get "Hidden")
  (`UserWidget.AddToViewport` (`self.ReloadWidget`) 0)
  (set `PlayerController.bShowMouseCursor` true (`GameplayStatics.GetPlayerController` 0))
  (bind _returnvalue_2 (`|CreateWidget` "/Game/BluePrints/FpsUI.FpsUI_C"))
  (`UserWidget.AddToViewport` _returnvalue_2 0))

(event `self.ReceiveEndPlay`
  (params (EndPlayReason :type "EEndPlayReason Enum" :default "ActorDestroyed"))
  (bind _foundwidgets (`WidgetBlueprintLibrary.GetAllWidgetsOfClass` "/Script/UMG.UserWidget"))
  (for _index (range (`KismetArrayLibrary.Array_Length` _foundwidgets))
    (`Widget.RemoveFromParent` (`KismetArrayLibrary.Array_Get` _foundwidgets _index))))

(fn `UserConstructionScript`)